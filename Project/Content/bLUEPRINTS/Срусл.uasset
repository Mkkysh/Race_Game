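; Checkpoint actor for a two-player racing game that records a respawn-style position and rotation on the player pawns.
; On any actor overlap, it copies its own location and rotation into the checkpoint variables of player 0's MyRace_GamePawn, then player 1's MyRace_GamePawn_2.
; The overlapping actor is never checked, so one overlap updates both players.
; The second update runs only if the first cast succeeds.
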(event EventBeginPlay)

(event Collision|EventActorBeginOverlap
  (params (OtherActor :type Actor%20Object%20Reference))
  (bind _asmy_race_game_pawn (Utilities|Casting|CastToMyRace_GamePawn (Game|Player|GetPlayerPawn 0)))
  (Variables|/Game/bLUEPRINTS/MyRace_GamePawn.MyRace_GamePawn_C|Setcheckpoint _asmy_race_game_pawn (Transformation|GetActorLocation))
  (Variables|/Game/bLUEPRINTS/MyRace_GamePawn.MyRace_GamePawn_C|SetCheckpointRot _asmy_race_game_pawn (Transformation|GetActorRotation))
  (bind _asmy_race_game_pawn_2 (Utilities|Casting|CastToMyRace_GamePawn_2 (Game|Player|GetPlayerPawn 1)))
  (Variables|/Game/bLUEPRINTS/MyRace_GamePawn_2.MyRace_GamePawn_2_C|SetCheckpoint_P _asmy_race_game_pawn_2 (Transformation|GetActorLocation))
  (Variables|/Game/bLUEPRINTS/MyRace_GamePawn_2.MyRace_GamePawn_2_C|SetrOTATION_P _asmy_race_game_pawn_2 (Transformation|GetActorRotation)))

(fn ConstructionScript)