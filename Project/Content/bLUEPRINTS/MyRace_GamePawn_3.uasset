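; A racing game pawn that handles pause menu input and two lights that act like brake lights.
; Escape or gamepad Special Right share a FlipFlop that creates the Pause_Menu widget, pauses and shows the cursor, then removes it and resumes.
; Holding S or Space Bar turns up the intensity of the left and right lights, and releasing sets it to zero.
; Driving logic is absent from these graphs.
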(event OnComponentActivated(SpringArm)
  (params (Component :type Actor%20Component%20Object%20Reference) (bReset :type Boolean)))

(event EventBeginPlay)

(event Collision|EventActorBeginOverlap
  (params (OtherActor :type Actor%20Object%20Reference)))

(event EventTick
  (params (DeltaSeconds :type Float%20%28single-precision%29)))

(event Input|KeyboardEvents|Escape
  (params (Key :type Key%20Structure :default "None"))
  (bind _returnvalue (Game|GetPlayerController 0))
  (:Pressed
    (Utilities|FlowControl|FlipFlop
      (:A
        (bind _returnvalue_2 (UserInterface|CreateWidget "/Game/Pause_menu/Pause_Menu.Pause_Menu_C"))
        (UserInterface|Viewport|AddtoViewport _returnvalue_2 0)
        (Input|SetInputModeUIOnly (Game|GetPlayerController 0) _returnvalue_2 "DoNotLock")
        (Class|WidgetBlueprintLibrary|SetFocustoGameViewport)
        (Game|SetGamePaused true)
        (Variables|/Script/Engine.PlayerController|SetbShowMouseCursor _returnvalue true)
        (Variables|/Script/Engine.PlayerController|SetbEnableMouseOverEvents _returnvalue false)
        (Variables|/Script/Engine.PlayerController|SetbEnableClickEvents _returnvalue false))
      (:B
        (Widget|RemovefromParent _returnvalue_2)
        (Input|SetInputModeGameOnly _returnvalue)
        (Class|WidgetBlueprintLibrary|SetFocustoGameViewport)
        (Game|SetGamePaused false)
        (Variables|/Script/Engine.PlayerController|SetbShowMouseCursor _returnvalue false)))))

(event Input|GamepadEvents|GamepadSpecialRight
  (params (Key :type Key%20Structure :default "None"))
  (bind _returnvalue (Game|GetPlayerController 0))
  (:Pressed
    (Utilities|FlowControl|FlipFlop
      (:A
        (bind _returnvalue_2 (UserInterface|CreateWidget "/Game/Pause_menu/Pause_Menu.Pause_Menu_C"))
        (UserInterface|Viewport|AddtoViewport _returnvalue_2 0)
        (Input|SetInputModeUIOnly (Game|GetPlayerController 0) _returnvalue_2 "DoNotLock")
        (Class|WidgetBlueprintLibrary|SetFocustoGameViewport)
        (Game|SetGamePaused true)
        (Variables|/Script/Engine.PlayerController|SetbShowMouseCursor _returnvalue true)
        (Variables|/Script/Engine.PlayerController|SetbEnableMouseOverEvents _returnvalue false)
        (Variables|/Script/Engine.PlayerController|SetbEnableClickEvents _returnvalue false))
      (:B
        (Widget|RemovefromParent _returnvalue_2)
        (Input|SetInputModeGameOnly _returnvalue)
        (Class|WidgetBlueprintLibrary|SetFocustoGameViewport)
        (Game|SetGamePaused false)
        (Variables|/Script/Engine.PlayerController|SetbShowMouseCursor _returnvalue false)))))

(event Input|KeyboardEvents|SpaceBar
  (params (Key :type Key%20Structure :default "None"))
  (bind _right_light (Variables|Default|GetRight_light))
  (:Pressed
    (Rendering|Components|Light|SetIntensity _right_light 5e+03))
  (:Released
    (Rendering|Components|Light|SetIntensity _right_light 0.0)))

(event Input|KeyboardEvents|S
  (params (Key :type Key%20Structure :default "None"))
  (bind _right_light (Variables|Default|GetRight_light))
  (:Pressed
    (Rendering|Components|Light|SetIntensity _right_light 5e+03))
  (:Released
    (Rendering|Components|Light|SetIntensity _right_light 0.0)))

(fn ConstructionScript)