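; Player controller, apparently for multiplayer racing, with car customization and spawning logic.
; Customization opens the Custom2 widget, pauses and shows the cursor; spawncar spawns one of two race pawns by Car0 at the current PlayerStart, possesses it and sets Magic.
; An index-driven chain matches PlayerStart tags and waits on Magic between players, but no event triggers it and BeginPlay is empty.
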(event Custom|Customization
  (bind _returnvalue (UserInterface|CreateWidget "/Game/Customisation/Custom2.Custom2_C" self))
  (UserInterface|Viewport|AddtoViewport _returnvalue 0)
  (Game|SetGamePaused true)
  (Variables|/Script/Engine.PlayerController|SetbShowMouseCursor self true)
  (if true
    _))

(event Custom|spawn%20car
  (bind _self self)
  (switch int (Variables|Default|Getcar0)
    (:0
      (bind _returnvalue (Game|SpawnActorfromClass "/Game/bLUEPRINTS/MyRace_GamePawn.MyRace_GamePawn_C" (Transformation|GetActorTransform (stale _array_element)) "AlwaysSpawn" 0 0))
      (Pawn|Possess _self _returnvalue)
      (Variables|Default|Set?Magic? true))
    (:1
      (bind _returnvalue_2 (Game|SpawnActorfromClass "/Game/bLUEPRINTS/MyRace_GamePawn_2.MyRace_GamePawn_2_C" (Transformation|GetActorTransform (stale _array_element)) "AlwaysSpawn" 0 0))
      (Pawn|Possess _self _returnvalue_2)
      (Variables|Default|Set?Magic? true))))

(event EventBeginPlay)

(fn ConstructionScript)

(fn GetPlayer
  (bind _outactors (Actor|GetAllActorsOfClass "/Script/Engine.PlayerStart"))
  (Variables|Default|SetOut%20Actors _outactors))