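; Player vehicle pawn for a racing game, handling pause, brake-style lights, engine audio, minimap and checkpoint reset.
; Escape or gamepad start toggles the pause menu through a FlipFlop, while brake and reverse-type inputs light two lights.
; Tick feeds absolute forward speed into the engine sound's RPM parameter.
; Possession by Player_For_Mult adds a per-player minimap, and Reset teleports the car to its stored checkpoint transform.
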(event EventBeginPlay
  (Variables|Default|SetMesh_M (Variables|Character|GetMesh)))

(event EventPossessed
  (params (NewController :type Controller%20Object%20Reference))
  (bind _asplayer_for_mult (Utilities|Casting|CastToPlayer_For_Mult NewController))
  (bind _returnvalue (UserInterface|CreateWidget "/Game/bLUEPRINTS/Widg_Minimap.Widg_Minimap_C" (Game|GetPlayerController (Variables|/Game/bLUEPRINTS/Player_For_Mult.Player_For_Mult_C|GetIndex _asplayer_for_mult))))
  (UserInterface|Viewport|AddtoPlayerScreen _returnvalue))

(event EventTick
  (params (DeltaSeconds :type Float%20%28single-precision%29))
  (CallFunction|Soundcar))

(event Input|ActionEvents|InputActionReset
  (params (Key :type Key%20Structure :default "None"))
  (:Pressed
    (Transformation|Teleport (Variables|Default|Getcheckpoint) (Variables|Default|GetCheckpointRot))))

(event Input|KeyboardEvents|Escape
  (params (Key :type Key%20Structure :default "None"))
  (bind _returnvalue (Game|GetPlayerController 0))
  (:Pressed
    (bind _asgame_mod_main_menu (Utilities|Casting|CastToGameModMainMenu (Game|GetGameMode)))
    (Variables|/Game/Main_Menu/GameModMainMenu.GameModMainMenu_C|SetPaused _asgame_mod_main_menu true)
    (Utilities|FlowControl|FlipFlop
      (:A
        (bind _returnvalue_2 (UserInterface|CreateWidget "/Game/Pause_menu/Pause_Menu.Pause_Menu_C"))
        (UserInterface|Viewport|AddtoViewport _returnvalue_2 0)
        (Input|SetInputModeUIOnly (Game|GetPlayerController 0) _returnvalue_2 "DoNotLock")
        (Class|WidgetBlueprintLibrary|SetFocustoGameViewport)
        (Game|SetGamePaused true)
        (Variables|/Script/Engine.PlayerController|SetbShowMouseCursor _returnvalue true)
        (Variables|/Script/Engine.PlayerController|SetbEnableMouseOverEvents _returnvalue false)
        (Variables|/Script/Engine.PlayerController|SetbEnableClickEvents _returnvalue false))
      (:B
        (Game|SetGamePaused false)
        (Widget|RemovefromParent _returnvalue_2)
        (Input|SetInputModeGameOnly _returnvalue)
        (Class|WidgetBlueprintLibrary|SetFocustoGameViewport)
        (Variables|/Script/Engine.PlayerController|SetbShowMouseCursor _returnvalue false)))))

(event Input|GamepadEvents|GamepadSpecialRight
  (params (Key :type Key%20Structure :default "None"))
  (bind _returnvalue (Game|GetPlayerController 0))
  (:Pressed
    (Utilities|FlowControl|FlipFlop
      (:A
        (bind _returnvalue_2 (UserInterface|CreateWidget "/Game/Pause_menu/Pause_Menu.Pause_Menu_C"))
        (UserInterface|Viewport|AddtoViewport _returnvalue_2 0)
        (Input|SetInputModeUIOnly (Game|GetPlayerController 0) _returnvalue_2 "DoNotLock")
        (Class|WidgetBlueprintLibrary|SetFocustoGameViewport)
        (Game|SetGamePaused true)
        (Variables|/Script/Engine.PlayerController|SetbShowMouseCursor _returnvalue true)
        (Variables|/Script/Engine.PlayerController|SetbEnableMouseOverEvents _returnvalue false)
        (Variables|/Script/Engine.PlayerController|SetbEnableClickEvents _returnvalue false))
      (:B
        (Game|SetGamePaused false)
        (Widget|RemovefromParent _returnvalue_2)
        (Input|SetInputModeGameOnly _returnvalue)
        (Class|WidgetBlueprintLibrary|SetFocustoGameViewport)
        (Variables|/Script/Engine.PlayerController|SetbShowMouseCursor _returnvalue false)))))

(event Input|KeyboardEvents|SpaceBar
  (params (Key :type Key%20Structure :default "None"))
  (bind _left_light (Variables|Default|GetLeft_Light))
  (:Pressed
    (Rendering|Components|Light|SetIntensity _left_light 5e+03))
  (:Released
    (Rendering|Components|Light|SetIntensity _left_light 0.0)))

(event Input|KeyboardEvents|S
  (params (Key :type Key%20Structure :default "None"))
  (bind _left_light (Variables|Default|GetLeft_Light))
  (:Pressed
    (Rendering|Components|Light|SetIntensity _left_light 5e+03))
  (:Released
    (Rendering|Components|Light|SetIntensity _left_light 0.0)))

(event Input|GamepadEvents|GamepadFaceButtonBottom
  (params (Key :type Key%20Structure :default "None"))
  (bind _left_light (Variables|Default|GetLeft_Light))
  (:Pressed
    (Rendering|Components|Light|SetIntensity _left_light 5e+03))
  (:Released
    (Rendering|Components|Light|SetIntensity _left_light 0.0)))

(event Input|GamepadEvents|GamepadLeftTrigger
  (params (Key :type Key%20Structure :default "None"))
  (bind _left_light (Variables|Default|GetLeft_Light))
  (:Pressed
    (Rendering|Components|Light|SetIntensity _left_light 5e+03))
  (:Released
    (Rendering|Components|Light|SetIntensity _left_light 0.0)))

(fn ConstructionScript)

(fn Soundcar
  (Audio|Parameter|SetFloatParameter (Variables|Default|GetEngineAudio) "RPM" (Math|Float|Absolute(Float) (Class|WheeledVehicleMovementComponent|GetForwardSpeed (Variables|Default|GetVehicleMovement))) :!class /Script/Engine.AudioComponent))